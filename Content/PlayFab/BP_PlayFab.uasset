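; PlayFab matchmaking actor that logs in with a fixed custom ID and pairs players into listen-server sessions.
; On Ticket input it creates a matchmaking ticket with the title player ID, then polls it on a looping timer until matched.
; Team A hosts an Advanced Sessions game tagged with the MatchId and opens TheMap; Team B waits briefly, then finds and joins that session.
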(event `OnFail`
  (params (error :type "PlayFabError Structure") (customData :type "Object Object Reference"))
  ;[1 1 1] Login
  (`self.FailLog` error))

(event `self.ReceiveBeginPlay`
  (`KismetSystemLibrary.ExecuteConsoleCommand` "Stat FPS" null)
  ;[1 1 1] Login
  (`self.EnableInput` (`GameplayStatics.GetPlayerControllerFromID` 0))
  (`PlayFabClientAPI.LoginWithCustomID` (make `ClientLoginWithCustomIDRequest` true "CustomIDDekstop") (delegate `On Login`) (delegate `OnFail`)))

(event `On Login`
  (params (result :type "ClientLoginResult Structure") (customData :type "Object Object Reference"))
  ;[1 1 1] Login
  (bind _output_get (set `self.PlayerId` (`.PlayFabId` (break `ClientLoginResult` result))))
  (`KismetSystemLibrary.PrintString` (`KismetStringLibrary.Concat_StrStr` "Player ID-> " _output_get))
  (`self.GetAccountInfo`))

(event `AccountInfoSuccess`
  (params (result :type "ClientGetAccountInfoResult Structure") (customData :type "Object Object Reference"))
  (bind _returnvalue (`PlayFabJsonObject.GetStringField` (`PlayFabJsonObject.GetObjectField` (`PlayFabJsonObject.GetObjectField` (`.AccountInfo` (break `ClientGetAccountInfoResult` result)) "TitleInfo") "TitlePlayerAccount") "Id"))
  ;[1 1 1] GetPlayerTitleId
  (`KismetSystemLibrary.PrintString` (`KismetStringLibrary.Concat_StrStr` "Title Player ID -> " _returnvalue))
  (set `self.PlayerTitle ID` _returnvalue))

(event `GetAccountInfo`
  ;[1 1 1] GetPlayerTitleId
  (`PlayFabClientAPI.GetAccountInfo` (make `ClientGetAccountInfoRequest` "" (`self.PlayerId`)) (delegate `AccountInfoSuccess`) (delegate `OnFailOnfo`)))

(event `OnFailOnfo`
  (params (error :type "PlayFabError Structure") (customData :type "Object Object Reference"))
  ;[1 1 1] GetPlayerTitleId
  (`self.FailLog` error))

(event `InputAction|Ticket`
  (params (Key :type "Key Structure"))
  (:`Pressed`
    (`self.CreateTicket` (`self.PlayerId`) (`self.QueueName`))))

(event `TicketCreated`
  (params (result :type "MultiplayerCreateMatchmakingTicketResult Structure") (customData :type "Object Object Reference"))
  (bind _output_get (set `self.Ticket Id` (`.TicketId` (break `MultiplayerCreateMatchmakingTicketResult` result))))
  (`KismetSystemLibrary.PrintString` (`KismetStringLibrary.Concat_StrStr` "TicketId -> " _output_get))
  (bind _returnvalue (`KismetSystemLibrary.K2_SetTimer` null "CheckMatchFound" 10.0 true))
  (set `self.SearchMatchUpdateTimerHandler` _returnvalue))

(event `CreateTicket`
  (params (PlayerID :type String) (QueueName :type String))
  (bind _creator_setting (`self.Creator Setting`))
  (`DestroySessionCallbackProxy.DestroySession` (`GameplayStatics.GetPlayerController` 0)
    (:`then`
      (set `self.Creator Setting` (`PlayFabJsonObject.ConstructJsonObject`))
      (set `self.Entity Key Setting` (`PlayFabJsonObject.ConstructJsonObject`))
      (`PlayFabJsonObject.SetStringField` _creator_setting "Id" (`self.PlayerTitle ID`))
      (`PlayFabJsonObject.SetStringField` _creator_setting "Type" "title_player_account")
      (`PlayFabJsonObject.SetStringField` _creator_setting "TypeString" "title_player_account")
      (`PlayFabJsonObject.SetObjectField` (`self.Entity Key Setting`) "Entity" (`self.Creator Setting`))
      (`PlayFabMultiplayerAPI.CreateMatchmakingTicket` (make `MultiplayerCreateMatchmakingTicketRequest` (`self.Entity Key Setting`) null 120 (`self.Members To Match With_0`) (`self.QueueName`)) (delegate `TicketCreated`) (delegate `MatchMakingFail`)))))

(event `MatchMakingFail`
  (params (error :type "PlayFabError Structure") (customData :type "Object Object Reference"))
  (`self.FailLog` error))

(event `GotMatchMakingTicket`
  (params (result :type "MultiplayerGetMatchmakingTicketResult Structure") (customData :type "Object Object Reference"))
  (bind (_cancellationreasonstring _created _creator _giveupafterseconds _matchid _members _memberstomatchwith _queuename _status) (break `MultiplayerGetMatchmakingTicketResult` result))
  (if (`KismetStringLibrary.EqualEqual_StrStr` _status "Matched")
    (`KismetSystemLibrary.K2_ClearAndInvalidateTimerHandle` (`self.SearchMatchUpdateTimerHandler`))
    (`self.GetMatch` _matchid _queuename)))

(event `GetMatchMakingTicket`
  (params (QueueName :type String) (TicketId :type String))
  (`PlayFabMultiplayerAPI.GetMatchmakingTicket` (make `MultiplayerGetMatchmakingTicketRequest` null false QueueName TicketId) (delegate `GotMatchMakingTicket`) (delegate `CantGetMatchMakingTicket`)))

(event `CantGetMatchMakingTicket`
  (params (error :type "PlayFabError Structure") (customData :type "Object Object Reference"))
  (`self.FailLog` error))

(event `GotMatch`
  (params (result :type "MultiplayerGetMatchResult Structure") (customData :type "Object Object Reference"))
  (bind (_matchid _members) (break `MultiplayerGetMatchResult` result))
  (bind _returnvalue (`GameplayStatics.GetPlayerController` 0))
  (`KismetSystemLibrary.PrintString` (`KismetStringLibrary.Concat_StrStr` "The MatchId -> " _matchid))
  (for _array_element _members
    (switch `string` (`PlayFabJsonObject.GetStringField` _array_element "TeamId")
      (:`TeamA`
        (bind _returnvalue_2 (`KismetStringLibrary.EqualEqual_StrStr` (`self.PlayerTitle ID`) (`PlayFabJsonObject.GetStringField` (`PlayFabJsonObject.GetObjectField` _array_element "Entity") "Id")))
        (if _returnvalue_2
          (`CreateSessionCallbackProxyAdvanced.CreateAdvancedSession` (`|MakeArray` (`AdvancedSessionsLibrary.MakeLiteralSessionPropertyString` "MatchId" _matchid)) (`GameplayStatics.GetPlayerController` 0)
            (:`OnSuccess`
              (`KismetSystemLibrary.PrintString` "Session Created" true true (struct :`R` 0.959213 :`G` 1.0 :`A` 1.0) 15.0)
              (`GameplayStatics.OpenLevel` "TheMap" true "?listen")))))
      (:`TeamB`
        (if _returnvalue_2
          (`KismetSystemLibrary.Delay` 5.0)
          (bind _results (`FindSessionsCallbackProxyAdvanced.FindSessionsAdvanced` _returnvalue 0 false "AllServers" (`|MakeArray` (`AdvancedSessionsLibrary.MakeLiteralSessionSearchProperty` (`AdvancedSessionsLibrary.MakeLiteralSessionPropertyString` "MatchId" _matchid) "Equals")))
            (:`OnSuccess`
              (`JoinSessionCallbackProxy.JoinSession` _returnvalue (`|GetArrayItem` _results)
                (:`OnSuccess`
                  (`KismetSystemLibrary.PrintString` "Session Joined" true true (struct :`R` 1.0 :`G` 0.796319 :`A` 1.0) 15.0))))))))))

(event `GetMatch`
  (params (MatchId :type String) (QueueName :type String))
  (`PlayFabMultiplayerAPI.GetMatch` (make `MultiplayerGetMatchRequest` null false MatchId QueueName) (delegate `GotMatch`) (delegate `FailedGetMatch`)))

(event `FailedGetMatch`
  (params (error :type "PlayFabError Structure") (customData :type "Object Object Reference")))

(event `SuccessQueueStat`
  (params (result :type "MultiplayerGetQueueStatisticsResult Structure") (customData :type "Object Object Reference")))

(event `GetqueueStaticstic`
  (`PlayFabMultiplayerAPI.GetQueueStatistics` (make `MultiplayerGetQueueStatisticsRequest` null "TestQ") (delegate `SuccessQueueStat`) (delegate `FailQueueStat`)))

(event `FailQueueStat`
  (params (error :type "PlayFabError Structure") (customData :type "Object Object Reference")))

(fn `CheckMatchFound`
  (`self.GetMatchMakingTicket` "TestQ" (`self.Ticket Id`)))

(fn `FailLog`
  (params (`Error Struct` :type "PlayFabError Structure"))
  (bind (_haserror _errorcode _errorname _errormessage _errordetails) (break `PlayFabError` `Error Struct`))
  (`KismetSystemLibrary.PrintString` _errorname)
  (`KismetSystemLibrary.PrintString` _errormessage)
  (`KismetSystemLibrary.PrintString` _errordetails))

(fn `GetPlayerID`
  (returns (PlayerTitleId :type String) (QueueName :type String))
  (return (`self.PlayerTitle ID`) (`self.QueueName`)))

(fn `Print`
  (`KismetSystemLibrary.PrintString` "Command Executed"))

(fn `UserConstructionScript`)